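; Inventory container component, with several per actor distinguished by ContainerType, each bound to its matching W_Container widget.
; Pickups try one priority container (hotbar) first, then the others, topping up the smallest stack or adding within space limits.
; Added items are hidden and attached to a Character owner's hand socket.
; Queries and consumption pool items by name across target container types, while Tick prints contents for debugging.
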(event `self.ReceiveBeginPlay`
  (`self.Innit Widget`)
  (`self.Random Color`))

(event `self.ReceiveTick`
  (params (DeltaSeconds :type "Float (single-precision)"))
  (`self.Print Item List`))

(event `/Game/AdditionalContent/Project_Modular_GBS/Blueprints/Interfaces/BPI_Container.Try Add Item`
  (params (`Item Ref` :type "/Game/AdditionalContent/Project_Modular_GBS/Blueprints/BP_Item Object Reference"))
  (`self.Global Add` `Item Ref`))

(event `/Game/AdditionalContent/Project_Modular_GBS/Blueprints/Interfaces/BPI_Container.Try Remove Item`
  (params (`Item Ref` :type "/Game/AdditionalContent/Project_Modular_GBS/Blueprints/BP_Item Object Reference"))
  (`self.Global Remove` `Item Ref`))

(fn `Add Directly`
  (params (`Item Ref` :type "/Game/AdditionalContent/Project_Modular_GBS/Blueprints/BP_Item Object Reference"))
  (returns (Added :type Boolean))
  (bind _item_ref (`local.Item Ref`))
  (if (>= (`self.Container Space`) (+ (`/Game/AdditionalContent/Project_Modular_GBS/Blueprints/Systems/Systems_Setup/DA_Item.Inventory Space` (`/Game/AdditionalContent/Project_Modular_GBS/Blueprints/BP_Item.Item Data` `Item Ref`)) (`self.Get Total Space` (`self.Content`))))
    (`KismetArrayLibrary.Array_Add` (`self.Content`) _item_ref)
    (message `/Game/AdditionalContent/Project_Modular_GBS/Blueprints/Interfaces/BPI_Container.Add Item Widget` (`self.Widget Ref`) (`/Game/AdditionalContent/Project_Modular_GBS/Blueprints/BP_Item.Get Widget` _item_ref))
    (message `/Game/AdditionalContent/Project_Modular_GBS/Blueprints/Interfaces/BPI_Item.Picked Up` _item_ref (`self.GetOwner`))
    (return true)
    (else
      (return false))))

(fn `Add Item To Container`
  (params (`Item Ref` :type "/Game/AdditionalContent/Project_Modular_GBS/Blueprints/BP_Item Object Reference"))
  (returns (Added :type Boolean) (Consumed :type Boolean))
  (locals (`Least Item` :type "/Game/AdditionalContent/Project_Modular_GBS/Blueprints/BP_Item Object Reference"))
  (bind (_found_any _items_ref) (`self.Query Container By Actor` `Item Ref`))
  (bind _least_item (`local.Least Item`))
  (set `local.Least Item` (`self.Get Least Quantity` _items_ref))
  (if _found_any
    (if (< (`/Game/AdditionalContent/Project_Modular_GBS/Blueprints/BP_Item.Quantity` _least_item) (`/Game/AdditionalContent/Project_Modular_GBS/Blueprints/Systems/Systems_Setup/DA_Item.Max Per Stack` (`/Game/AdditionalContent/Project_Modular_GBS/Blueprints/BP_Item.Item Data` _least_item)))
      (`self.Collect Item` (`local.Least Item`) (`local.Item Ref`))
      (return false true)
      (elif (`/Game/AdditionalContent/Project_Modular_GBS/Blueprints/Systems/Systems_Setup/DA_Item.Is Unique` (`/Game/AdditionalContent/Project_Modular_GBS/Blueprints/BP_Item.Item Data` (`local.Item Ref`)))
        (return false false)
        (else
          (bind _added (`self.Add Directly` (`local.Item Ref`)))
          (return _added false))))
    (else
      (bind _added_2 (`self.Add Directly` (`local.Item Ref`)))
      (return _added_2 false))))

(fn `Attach Item`
  (params (`Item Ref` :type "/Game/AdditionalContent/Project_Modular_GBS/Blueprints/BP_Item Object Reference"))
  (returns (Attached :type Boolean))
  (bind (_ischaracter _character) (`self.Get System Owner`))
  (bind _returnvalue (select `bool` false :`false` "hand_rSocket" :`true` "hand_lSocket" :!type "Name"))
  (bind _mesh (`Character.Mesh` _character))
  (if _ischaracter
    (`Actor.K2_AttachToComponent` `Item Ref` _mesh _returnvalue "SnapToTarget" "SnapToTarget" "SnapToTarget" true)
    (`SceneComponent.K2_AttachToComponent` (`/Game/AdditionalContent/Project_Modular_GBS/Blueprints/BP_Item.Static Mesh` `Item Ref`) _mesh _returnvalue "SnapToTarget" "SnapToTarget" "SnapToTarget" true)
    (return true)
    (else
      (return false))))

(fn `Collect Item`
  (params (`Current Item` :type "/Game/AdditionalContent/Project_Modular_GBS/Blueprints/BP_Item Object Reference") (`Other Item` :type "/Game/AdditionalContent/Project_Modular_GBS/Blueprints/BP_Item Object Reference"))
  (locals (Consumed :type Integer :default 0))
  (bind _other_item (`local.Other Item`))
  (bind _output_get (set `local.Consumed` (`KismetMathLibrary.Clamp` (- (`/Game/AdditionalContent/Project_Modular_GBS/Blueprints/Systems/Systems_Setup/DA_Item.Max Per Stack` (`/Game/AdditionalContent/Project_Modular_GBS/Blueprints/BP_Item.Item Data` `Current Item`)) (`/Game/AdditionalContent/Project_Modular_GBS/Blueprints/BP_Item.Quantity` `Current Item`)) 0 (`/Game/AdditionalContent/Project_Modular_GBS/Blueprints/BP_Item.Quantity` `Other Item`))))
  (bind _output_get_2 (set `/Game/AdditionalContent/Project_Modular_GBS/Blueprints/BP_Item.Quantity` (+ (stale _output_get_2) _output_get) `Current Item`))
  (bind _output_get_3 (set `/Game/AdditionalContent/Project_Modular_GBS/Blueprints/BP_Item.Quantity` (- (stale _output_get_3) _output_get) _other_item))
  (message `/Game/AdditionalContent/Project_Modular_GBS/Blueprints/Interfaces/BPI_Item.Item Quantity Updated` _other_item)
  (message `/Game/AdditionalContent/Project_Modular_GBS/Blueprints/Interfaces/BPI_Item.Item Quantity Updated` (`local.Current Item`))
  (return))

(fn `Consume Item`
  (params (`Item Ref` :type "/Game/AdditionalContent/Project_Modular_GBS/Blueprints/Systems/Systems_Setup/DA_Item Object Reference") (`To Consume` :type Integer) (`Target Types` :type "Array of /Game/AdditionalContent/Project_Modular_GBS/Blueprints/Systems/Systems_Setup/E_Container_Type Enum (by ref)"))
  (returns (`Total Consumed` :type Integer) (`Any Consumed` :type Boolean) (`Full Consume` :type Boolean))
  (locals (`To Remve` :type Integer) (`Total Consumed 1` :type Integer) (`To be consumed` :type "Array of /Game/AdditionalContent/Project_Modular_GBS/Blueprints/BP_Item Object Reference") (Current :type Integer :default 0))
  (bind _total_consumed_1 (`local.Total Consumed 1`))
  (bind _least_quantity_item (`self.Get Least Quantity` (`local.To be consumed`)))
  (bind _quantity (`/Game/AdditionalContent/Project_Modular_GBS/Blueprints/BP_Item.Quantity` _least_quantity_item))
  (set `local.To Remve` `To Consume`)
  (bind _output_get (set `local.To be consumed` (`.Items Ref` (`self.Query Container DA` `Item Ref` (`self.Get Compined Items` `Target Types`)))))
  (while (not (or (<= (`local.To Remve`) 0) (<= (`self.Get Total Quantity` _output_get) 0)))
    (`KismetSystemLibrary.PrintString` "Hello")
    (bind _output_get_2 (set `local.Current` (`KismetMathLibrary.Clamp` (`local.To Remve`) 0 _quantity)))
    (bind _output_get_3 (set `local.Total Consumed 1` (+ (stale _output_get_3) _output_get_2)))
    (set `/Game/AdditionalContent/Project_Modular_GBS/Blueprints/BP_Item.Quantity` (- _quantity (`local.Current`)) _least_quantity_item)
    (message `/Game/AdditionalContent/Project_Modular_GBS/Blueprints/Interfaces/BPI_Item.Item Quantity Updated` _least_quantity_item)
    (bind _output_get_4 (set `local.To Remve` (- (stale _output_get_4) (`local.Current`)))))
  (return (`local.Total Consumed 1`) (> _total_consumed_1 0) (== _total_consumed_1 (`local.To Consume`))))

(fn `Consume Request`
  (params (`Item DA Ref` :type "/Game/AdditionalContent/Project_Modular_GBS/Blueprints/Systems/Systems_Setup/DA_Item Object Reference") (Quantity :type Integer) (`Consume/Pay` :type Boolean) (`Target Containers` :type "Array of /Game/AdditionalContent/Project_Modular_GBS/Blueprints/Systems/Systems_Setup/E_Container_Type Enum (by ref)" :default _))
  (returns (Granted :type Integer))
  (bind _consuemd (`self.Try Consume` `Item DA Ref` Quantity `Consume/Pay` `Target Containers`))
  (return _consuemd))

(fn `Get Compined Items`
  (params (`Target Containers` :type "Array of /Game/AdditionalContent/Project_Modular_GBS/Blueprints/Systems/Systems_Setup/E_Container_Type Enum (by ref)"))
  (returns (Total1 :type "Array of /Game/AdditionalContent/Project_Modular_GBS/Blueprints/BP_Item Object Reference"))
  (locals (Total :type "Array of /Game/AdditionalContent/Project_Modular_GBS/Blueprints/BP_Item Object Reference"))
  (for _array_element (`Actor.K2_GetComponentsByClass` (`self.GetOwner`) "Container_System_C")
    (if (`KismetArrayLibrary.Array_Contains` `Target Containers` (`/Game/AdditionalContent/Project_Modular_GBS/Blueprints/Systems/Container_System.Container Type` _array_element))
      (`KismetArrayLibrary.Array_Append` (`local.Total`) (`/Game/AdditionalContent/Project_Modular_GBS/Blueprints/Systems/Container_System.Content` _array_element) :!label _label)
      (elif (`KismetArrayLibrary.Array_Contains` `Target Containers` "NewEnumerator3")
        (goto _label))))
  (return (`local.Total`)))

(fn `Get Container`
  (params (Type :type "/Game/AdditionalContent/Project_Modular_GBS/Blueprints/Systems/Systems_Setup/E_Container_Type Enum" :default "NewEnumerator0"))
  (returns (Found :type Boolean) (Container :type "/Game/AdditionalContent/Project_Modular_GBS/Blueprints/Systems/Container_System Object Reference"))
  (for _array_element (`Actor.K2_GetComponentsByClass` (`self.GetOwner`) "Container_System_C")
    (if (`|EnumEquality` (`/Game/AdditionalContent/Project_Modular_GBS/Blueprints/Systems/Container_System.Container Type` _array_element) Type)
      (return true _array_element)))
  (return false null))

(fn `Get Least Quantity`
  (params (Items :type "Array of /Game/AdditionalContent/Project_Modular_GBS/Blueprints/BP_Item Object Reference"))
  (returns (`Least Quantity Item` :type "/Game/AdditionalContent/Project_Modular_GBS/Blueprints/BP_Item Object Reference"))
  (locals (Least :type Integer :default 0) (`Least Item2` :type "/Game/AdditionalContent/Project_Modular_GBS/Blueprints/BP_Item Object Reference"))
  (for _array_element Items
    (`local.Least Item2`
      (:`then`
        (bind _quantity (`/Game/AdditionalContent/Project_Modular_GBS/Blueprints/BP_Item.Quantity` _array_element))
        (if (< _quantity (`local.Least`))
          (set `local.Least Item2` _array_element)
          (set `local.Least` _quantity)))
      (:`else`
        (set `local.Least Item2` _array_element)
        (set `local.Least` _quantity))))
  (return (`local.Least Item2`)))

(fn `Get System Owner`
  (returns (IsCharacter :type Boolean) (Character :type "Character Object Reference"))
  (bind _ascharacter (cast `Character` (`self.GetOwner`))
    (:`then`
      (return true _ascharacter))
    (:`CastFailed`
      (return false null))))

(fn `Get Total Quantity`
  (params (Items :type "Array of /Game/AdditionalContent/Project_Modular_GBS/Blueprints/BP_Item Object Reference"))
  (returns (Total :type Integer) (Infinit :type Boolean))
  (locals (`Total Count` :type Integer :default 0) (`Infifnt Item` :type Boolean :default false))
  (for _array_element Items
    (`/Engine/EditorBlueprintResources/StandardMacros.IsValid` _array_element
      (:`Is Valid`
        (bind _output_get (set `local.Total Count` (+ (stale _output_get) (`/Game/AdditionalContent/Project_Modular_GBS/Blueprints/BP_Item.Quantity` _array_element))))
        (if (`/Game/AdditionalContent/Project_Modular_GBS/Blueprints/Systems/Systems_Setup/DA_Item.Infinit` (`/Game/AdditionalContent/Project_Modular_GBS/Blueprints/BP_Item.Item Data` _array_element))
          (set `local.Infifnt Item` true)))))
  (return (`local.Total Count`) (`local.Infifnt Item`)))

(fn `Get Total Space`
  (params (Items :type "Array of /Game/AdditionalContent/Project_Modular_GBS/Blueprints/BP_Item Object Reference"))
  (returns (Total :type Integer))
  (locals (`Total ` :type Integer :default 0) (`Infifnt Item` :type Boolean :default false))
  (for _array_element Items
    (bind _output_get (set `local.Total ` (+ (stale _output_get) (`/Game/AdditionalContent/Project_Modular_GBS/Blueprints/Systems/Systems_Setup/DA_Item.Inventory Space` (`/Game/AdditionalContent/Project_Modular_GBS/Blueprints/BP_Item.Item Data` _array_element))))))
  (return (`local.Total `)))

(fn `Get Unique Names`
  (returns (`Unique Names` :type "Array of Text"))
  (locals (`Unique Names2` :type "Array of Text"))
  (bind _unique_names2 (`local.Unique Names2`))
  (for _array_element (`self.Content`)
    (bind _asbp_item (cast `/Game/AdditionalContent/Project_Modular_GBS/Blueprints/BP_Item` _array_element))
    (`KismetArrayLibrary.Array_AddUnique` _unique_names2 (`/Game/AdditionalContent/Project_Modular_GBS/Blueprints/Systems/Systems_Setup/DA_Item.Name` (`/Game/AdditionalContent/Project_Modular_GBS/Blueprints/BP_Item.Item Data` _asbp_item)))
    (return _unique_names2)))

(fn `Global Add`
  (params (`Item Ref 1` :type "/Game/AdditionalContent/Project_Modular_GBS/Blueprints/BP_Item Object Reference"))
  (returns (Success :type Boolean))
  ;[1 1 1] This is here to priorities picking up the item to the hotbar over any other container on the player
  (bind (_added _attached _consumed) (`self.Try add` (`.Container` (`self.Get Container` "NewEnumerator0")) `Item Ref 1`))
  (if (or _added _consumed)
    (return true)
    (else
      ;[1 1 1] If not picked up try to pick it up to the first available container
      (for _array_element (`Actor.K2_GetComponentsByClass` (`self.GetOwner`) "Container_System_C")
        (bind (_added_2 _attached_2 _consumed_2) (`self.Try add` _array_element (`local.Item Ref 1`)))
        (if (or _added_2 _consumed_2)
          (return true)))
      (return false))))

(fn `Global Remove`
  (params (Item :type "/Game/AdditionalContent/Project_Modular_GBS/Blueprints/BP_Item Object Reference (by ref)"))
  (returns (Removed :type Boolean))
  (for _array_element (`Actor.K2_GetComponentsByClass` (`self.GetOwner`) "Container_System_C")
    (bind _returnvalue (`KismetArrayLibrary.Array_RemoveItem` (`/Game/AdditionalContent/Project_Modular_GBS/Blueprints/Systems/Container_System.Content` _array_element) Item))
    (if _returnvalue
      (return true)))
  (return false))

(fn `Innit Widget`
  ;[1 1 1] Comment
  (bind _foundwidgets (`WidgetBlueprintLibrary.GetAllWidgetsOfClass` "/Game/AdditionalContent/Project_Modular_GBS/Default_Demo_Widgets/W_Container.W_Container_C" false))
  (for _array_element _foundwidgets
    (if (`|EnumEquality` (`/Game/AdditionalContent/Project_Modular_GBS/Default_Demo_Widgets/W_Container.Container Type` _array_element) (`self.Container Type`))
      (set `self.Widget Ref` _array_element))))

(fn `Print Item List`
  (for _array_element (`self.Content`)
    (`KismetSystemLibrary.PrintString` (`KismetTextLibrary.Conv_TextToString` (`|FormatText` "{0} {1}" (`/Game/AdditionalContent/Project_Modular_GBS/Blueprints/BP_Item.Quantity` _array_element) (`/Game/AdditionalContent/Project_Modular_GBS/Blueprints/Systems/Systems_Setup/DA_Item.Name` (`/Game/AdditionalContent/Project_Modular_GBS/Blueprints/BP_Item.Item Data` _array_element)))) true true (`self.Print Color`) 0.0)))

(fn `Query Container By Actor`
  (params (`Item Ref` :type "/Game/AdditionalContent/Project_Modular_GBS/Blueprints/BP_Item Object Reference (by ref)"))
  (returns (`Found Any` :type Boolean) (`Items Ref` :type "Array of /Game/AdditionalContent/Project_Modular_GBS/Blueprints/BP_Item Object Reference"))
  (locals (`Items Found` :type "Array of /Game/AdditionalContent/Project_Modular_GBS/Blueprints/BP_Item Object Reference") (`Any Items Found` :type Boolean :default false))
  (for _array_element (`self.Content`)
    (if (`KismetTextLibrary.EqualEqual_TextText` (`/Game/AdditionalContent/Project_Modular_GBS/Blueprints/Systems/Systems_Setup/DA_Item.Name` (`/Game/AdditionalContent/Project_Modular_GBS/Blueprints/BP_Item.Item Data` _array_element)) (`/Game/AdditionalContent/Project_Modular_GBS/Blueprints/Systems/Systems_Setup/DA_Item.Name` (`/Game/AdditionalContent/Project_Modular_GBS/Blueprints/BP_Item.Item Data` `Item Ref`)))
      (`KismetArrayLibrary.Array_Add` (`local.Items Found`) _array_element)
      (set `local.Any Items Found` true)))
  (return (`local.Any Items Found`) (`local.Items Found`)))

(fn `Query Container by Index`
  (params (`Item Index` :type Integer))
  (returns (Found :type Boolean) (`Item Ref` :type "/Game/AdditionalContent/Project_Modular_GBS/Blueprints/BP_Item Object Reference"))
  (bind _output (`|GetArrayItem` (`self.Content`) `Item Index`))
  (`/Engine/EditorBlueprintResources/StandardMacros.IsValid` _output
    (:`Is Valid`
      (return true _output))
    (:`Is Not Valid`
      (return false null))))

(fn `Query Container DA`
  (params (`Item DA Ref` :type "/Game/AdditionalContent/Project_Modular_GBS/Blueprints/Systems/Systems_Setup/DA_Item Object Reference (by ref)") (Array :type "Array of /Game/AdditionalContent/Project_Modular_GBS/Blueprints/BP_Item Object Reference"))
  (returns (`Found Any` :type Boolean) (`Items Ref` :type "Array of /Game/AdditionalContent/Project_Modular_GBS/Blueprints/BP_Item Object Reference"))
  (locals (`Items Found` :type "Array of /Game/AdditionalContent/Project_Modular_GBS/Blueprints/BP_Item Object Reference") (`Any Items Found` :type Boolean :default false))
  (for _array_element Array
    (`/Engine/EditorBlueprintResources/StandardMacros.IsValid` `Item DA Ref`
      (:`Is Valid`
        (if (`KismetTextLibrary.EqualEqual_TextText` (`/Game/AdditionalContent/Project_Modular_GBS/Blueprints/Systems/Systems_Setup/DA_Item.Name` (`/Game/AdditionalContent/Project_Modular_GBS/Blueprints/BP_Item.Item Data` _array_element)) (`/Game/AdditionalContent/Project_Modular_GBS/Blueprints/Systems/Systems_Setup/DA_Item.Name` `Item DA Ref`))
          (`KismetArrayLibrary.Array_Add` (`local.Items Found`) _array_element)
          (set `local.Any Items Found` true)))
      (:`Is Not Valid`
        (`KismetSystemLibrary.PrintString` "Query Error" true true (struct :`R` 1.0 :`G` 0.033822 :`A` 1.0))
        (return false))))
  (return (`local.Any Items Found`) (`local.Items Found`)))

(fn `Query Item`
  (params (`Item DA Ref` :type "/Game/AdditionalContent/Project_Modular_GBS/Blueprints/Systems/Systems_Setup/DA_Item Object Reference") (`Target Containers` :type "Array of /Game/AdditionalContent/Project_Modular_GBS/Blueprints/Systems/Systems_Setup/E_Container_Type Enum (by ref)" :default _))
  (returns (Available :type Integer))
  (return (`self.Get Total Quantity` (`.Items Ref` (`self.Query Container DA` `Item DA Ref` (`self.Get Compined Items` `Target Containers`))))))

(fn `Random Color`
  (set `self.Print Color` (make `LinearColor` (`KismetMathLibrary.Conv_BoolToDouble` (`KismetMathLibrary.RandomBool`)) (`KismetMathLibrary.Conv_BoolToDouble` (`KismetMathLibrary.RandomBool`)) (`KismetMathLibrary.Conv_BoolToDouble` (`KismetMathLibrary.RandomBool`)) 1.0)))

(fn `Try add`
  (params (`Item Ref 1` :type "/Game/AdditionalContent/Project_Modular_GBS/Blueprints/BP_Item Object Reference"))
  (returns (Added :type Boolean) (Attached :type Boolean) (Consumed :type Boolean))
  (bind _item_ref_1 (`local.Item Ref 1`))
  (if (`self.Contains Holdables Only`)
    (if (`/Game/AdditionalContent/Project_Modular_GBS/Blueprints/Systems/Systems_Setup/DA_Item.Holdable` (`/Game/AdditionalContent/Project_Modular_GBS/Blueprints/BP_Item.Item Data` `Item Ref 1`))
      _
      (else
        (return false false false))))
  (bind (_added _consumed) (`self.Add Item To Container` (`local.Item Ref 1`)))
  (if _added
    (`Actor.SetActorHiddenInGame` _item_ref_1 true)
    (`Actor.SetActorEnableCollision` _item_ref_1 false)
    (bind _attached (`self.Attach Item` _item_ref_1))
    (if _attached
      (return true true false)
      (else
        (return true false false)))
    (elif _consumed
      (return false false true)
      (else
        (return false false false)))))

(fn `Try Consume`
  (params (`Item Ref` :type "/Game/AdditionalContent/Project_Modular_GBS/Blueprints/Systems/Systems_Setup/DA_Item Object Reference (by ref)") (`Consume Quantity` :type Integer) (`Consume/Pay` :type Boolean) (`Target Containers` :type "Array of /Game/AdditionalContent/Project_Modular_GBS/Blueprints/Systems/Systems_Setup/E_Container_Type Enum (by ref)"))
  (returns (Consuemd :type Integer) (`Consuemd Any` :type Boolean) (`Full Consume` :type Boolean))
  (locals (`Item Quantity` :type Integer :default 0) (`To be consumed` :type "Array of /Game/AdditionalContent/Project_Modular_GBS/Blueprints/BP_Item Object Reference"))
  (bind _consume_quantity (`local.Consume Quantity`))
  (bind (_found_any _items_ref) (`self.Query Container DA` `Item Ref` (`self.Get Compined Items` `Target Containers`)))
  (bind (_total _infinit) (`self.Get Total Quantity` _items_ref))
  (if _found_any
    (if _infinit
      (return `Consume Quantity` true true)
      (else
        (if (`local.Consume/Pay`)
          _
          (elif (<= _consume_quantity _total)
            _
            (else
              (return 0 false false))))
        (bind (_total_consumed _any_consumed _full_consume) (`self.Consume Item` (`local.Item Ref`) _consume_quantity `Target Containers`))
        (return _total_consumed _any_consumed _full_consume)))
    (else
      (return 0 false false))))