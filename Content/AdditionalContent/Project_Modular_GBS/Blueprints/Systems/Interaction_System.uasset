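; Interaction component that shows key-and-action prompts for its owner and a target actor, and picks up items.
; Target prompts use a lazily created screen-space widget component, rebuilt when the hovered actor changes and otherwise moved to that actor's Interaction_System.
; Owner prompts fill an existing W_Owner_Interactions widget; both sets come from each component's action maps via interface query.
; IA_Interact or DefaultInteraction sends the hovered BP_Item to the owner's Container_System.
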(event `EnhancedInput|/Game/AdditionalContent/Project_Modular_GBS/Blueprints/Player/Input/IA_Interact`
  (params (ActionValue :type Boolean) (ElapsedSeconds :type "Float (double-precision)") (TriggeredSeconds :type "Float (double-precision)") (InputAction :type "InputAction Object Reference" :default "/Game/AdditionalContent/Project_Modular_GBS/Blueprints/Player/Input/IA_Interact.IA_Interact"))
  (:`Started`
    (`self.Interact` (`self.GetOwner`) (`self.Hovered Actor`))))

(event `/Game/AdditionalContent/Project_Modular_GBS/Blueprints/Interfaces/BPI_Interact.Default Interaction`
  (params (`Interactor Ref` :type "Actor Object Reference"))
  (`self.Interact` `Interactor Ref` (`self.Hovered Actor`)))

(event `/Game/AdditionalContent/Project_Modular_GBS/Blueprints/Interfaces/BPI_Interact.Show All Interactions`
  (params (`Actor Ref` :type "Actor Object Reference") (`Owner/External` :type Boolean))
  (bind _returnvalue (`Actor.GetComponentByClass` `Actor Ref` "Interaction_System_C"))
  (bind _interaction_widget_ref (`self.Interaction Widget Ref`))
  (if `Owner/External`
    (`/Engine/EditorBlueprintResources/StandardMacros.IsValid` _returnvalue
      (:`Is Valid`
        (bind _owner_actions (`self.Get Owner Actions` (`self.GetOwner`)))
        (`self.Update Owner Widget` _owner_actions))
      (:`Is Not Valid`
        (`self.Hide All Interactions` true)))
    (else
      (`/Engine/EditorBlueprintResources/StandardMacros.IsValid` _returnvalue
        (:`Is Valid`
          (bind (_new _external_actions) (`self.Get External Actions` `Actor Ref`))
          (`self.Create World Widget`)
          (if _new
            (`self.Update External Widget` _external_actions)
            (else
              (`self.K2_SetWorldLocation` _interaction_widget_ref (`self.K2_GetComponentLocation` _returnvalue) false false)
              (`self.SetHiddenInGame` _interaction_widget_ref false false))))
        (:`Is Not Valid`
          (`self.Hide All Interactions` false)
          (set `self.Hovered Actor` null))))))

(event `/Game/AdditionalContent/Project_Modular_GBS/Blueprints/Interfaces/BPI_Interact.Hide All Interactions`
  (params (`Owner/External` :type Boolean))
  (if `Owner/External`
    (`self.Clear Owner`)
    (else
      (bind _interaction_widget_ref (`self.Interaction Widget Ref`)
        (:`then`
          (`self.SetHiddenInGame` _interaction_widget_ref true false))
        (:`else`)))))

(event `/Game/AdditionalContent/Project_Modular_GBS/Blueprints/Interfaces/BPI_Interact.Update Interactions`
  (params (`Owner Actions` :type "Map of Key Structure to String") (`External Actions` :type "Map of Key Structure to String"))
  (set `self.Owner Interactions` `Owner Actions`)
  (set `self.External Actions` `External Actions`))

(fn `Clear Owner`
  (bind _foundwidgets (`WidgetBlueprintLibrary.GetAllWidgetsOfClass` "/Game/AdditionalContent/Project_Modular_GBS/Default_Demo_Widgets/W_Owner_Interactions.W_Owner_Interactions_C" false))
  (if (not (`KismetArrayLibrary.Array_IsEmpty` _foundwidgets))
    (`/Game/AdditionalContent/Project_Modular_GBS/Default_Demo_Widgets/W_Interactions.Clear` (`|GetArrayItem` _foundwidgets))))

(fn `Create World Widget`
  (bind _interaction_widget_ref (`self.Interaction Widget Ref`))
  (`self.Interaction Widget Ref`
    (:`then`
      (return))
    (:`else`
      (bind _returnvalue (`|AddComponentByClass` (`self.GetOwner`) "/Script/UMG.WidgetComponent" true (`self.GetRelativeTransform`)))
      (set `self.Interaction Widget Ref` _returnvalue)
      (`PrimitiveComponent.SetCollisionEnabled` _interaction_widget_ref "NoCollision")
      (`WidgetComponent.SetDrawAtDesiredSize` _interaction_widget_ref true)
      (`WidgetComponent.SetWidgetSpace` _interaction_widget_ref "Screen")
      (bind _returnvalue_2 (`|CreateWidget` "/Game/AdditionalContent/Project_Modular_GBS/Default_Demo_Widgets/W_Interactions.W_Interactions_C"))
      (bind _output_get (set `self.Widget Ref` _returnvalue_2))
      (`WidgetComponent.SetWidget` _interaction_widget_ref _output_get)
      (return))))

(fn `Get Container`
  (params (Type :type "/Game/AdditionalContent/Project_Modular_GBS/Blueprints/Systems/Systems_Setup/E_Container_Type Enum" :default "NewEnumerator0"))
  (returns (Found :type Boolean) (Container :type "/Game/AdditionalContent/Project_Modular_GBS/Blueprints/Systems/Container_System Object Reference"))
  (for _array_element (`Actor.K2_GetComponentsByClass` (`self.GetOwner`) "/Game/AdditionalContent/Project_Modular_GBS/Blueprints/Systems/Container_System.Container_System_C")
    (if (`|EnumEquality` (`/Game/AdditionalContent/Project_Modular_GBS/Blueprints/Systems/Container_System.Container Type` _array_element) Type)
      (return true _array_element)))
  (return false null))

(fn `Get External Actions`
  (params (`Actor ref 1` :type "Actor Object Reference"))
  (returns (New :type Boolean) (`External Actions` :type "Map of Key Structure to String"))
  (if (!= `Actor ref 1` (`self.Hovered Actor`))
    (bind _output_get (set `self.Hovered Actor` `Actor ref 1`))
    (bind (_owner_actions _external_actions) (message `/Game/AdditionalContent/Project_Modular_GBS/Blueprints/Interfaces/BPI_Interact.Query Actions` (`Actor.GetComponentByClass` _output_get "Interaction_System_C")))
    (return true _external_actions)
    (else
      (return false))))

(fn `Get Owner Actions`
  (params (`Actor Ref 1` :type "Actor Object Reference"))
  (returns (`Owner Actions` :type "Map of Key Structure to String"))
  (bind _owner_actions (message `/Game/AdditionalContent/Project_Modular_GBS/Blueprints/Interfaces/BPI_Interact.Query Actions` (`Actor.GetComponentByClass` `Actor Ref 1` "Interaction_System_C")))
  (return _owner_actions))

(fn `Interact`
  (params (`Interactor Ref` :type "Actor Object Reference") (`Other Actor Ref` :type "Object Object Reference"))
  (bind _asbp_item (cast `/Game/AdditionalContent/Project_Modular_GBS/Blueprints/BP_Item` `Other Actor Ref`))
  (message `/Game/AdditionalContent/Project_Modular_GBS/Blueprints/Interfaces/BPI_Container.Try Add Item` (`Actor.GetComponentByClass` (`self.GetOwner`) "/Game/AdditionalContent/Project_Modular_GBS/Blueprints/Systems/Container_System.Container_System_C") _asbp_item))

(fn `Query Actions`
  (returns (`Owner Actions` :type "Map of Key Structure to String") (`External Actions` :type "Map of Key Structure to String"))
  (return (`self.Owner Interactions`) (`self.External Actions`)))

(fn `Update External Widget`
  (params (`External Actions` :type "Map of Key Structure to String"))
  (bind _widget_ref (`self.Widget Ref`))
  (bind _keys (`BlueprintMapLibrary.Map_Keys` `External Actions`))
  (if (`KismetArrayLibrary.Array_IsEmpty` _keys)
    (`/Game/AdditionalContent/Project_Modular_GBS/Default_Demo_Widgets/W_Interactions.Clear` _widget_ref)
    (else
      (`/Game/AdditionalContent/Project_Modular_GBS/Default_Demo_Widgets/W_Interactions.Clear` _widget_ref)
      (`self.SetHiddenInGame` (`self.Interaction Widget Ref`) false false)
      (bind _values (`BlueprintMapLibrary.Map_Values` `External Actions`))
      (for (_array_element _array_index) _keys
        (bind _returnvalue (`|CreateWidget` "/Game/AdditionalContent/Project_Modular_GBS/Default_Demo_Widgets/W_Action.W_Action_C" null (`|GetArrayItem` _values _array_index) (`KismetTextLibrary.Conv_TextToString` (`KismetInputLibrary.Key_GetDisplayName` _array_element))))
        (`/Game/AdditionalContent/Project_Modular_GBS/Default_Demo_Widgets/W_Interactions.Add Action` (`self.Widget Ref`) _returnvalue)))))

(fn `Update Owner Widget`
  (params (`Owner Actions 1` :type "Map of Key Structure to String"))
  (bind _foundwidgets (`WidgetBlueprintLibrary.GetAllWidgetsOfClass` "/Game/AdditionalContent/Project_Modular_GBS/Default_Demo_Widgets/W_Owner_Interactions.W_Owner_Interactions_C" false))
  (if (`KismetArrayLibrary.Array_IsNotEmpty` _foundwidgets)
    (bind _output (`|GetArrayItem` _foundwidgets))
    (`/Game/AdditionalContent/Project_Modular_GBS/Default_Demo_Widgets/W_Interactions.Clear` _output)
    (bind _keys (`BlueprintMapLibrary.Map_Keys` `Owner Actions 1`))
    (for _array_element _keys
      (bind _returnvalue (`|CreateWidget` "/Game/AdditionalContent/Project_Modular_GBS/Default_Demo_Widgets/W_Action.W_Action_C" null (`BlueprintMapLibrary.Map_Find` (`local.Owner Actions 1`) _array_element) (`KismetTextLibrary.Conv_TextToString` (`KismetInputLibrary.Key_GetDisplayName` _array_element))))
      (`/Game/AdditionalContent/Project_Modular_GBS/Default_Demo_Widgets/W_Interactions.Add Action` _output _returnvalue))))

(fn `Update Widget Position`
  (params (`New Location` :type "Vector Structure")))