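; Trace System component providing multi-hit object line traces from view center, between two points, or from a point toward the crosshair, with optional debug drawing.
; View origin comes from the instigator's camera, falling back to the owner's camera, then actor transform.
; Crosshair traces first find the view-center target, then re-trace from the given point toward it.
; Point-to-point and crosshair traces add random angular spread derived from MOA accuracy.
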(fn `Calculate Accuracy`
  (params (Start :type "Vector Structure") (End :type "Vector Structure") (`Accuracy MOA` :type "Float (double-precision)"))
  (returns (`New End` :type "Vector Structure"))
  (bind _returnvalue (/ `Accuracy MOA` 60.0 0.5))
  (bind _returnvalue_2 (* _returnvalue -1.0))
  (return (+ (`KismetMathLibrary.GreaterGreater_VectorRotator` (- End Start) (`KismetMathLibrary.MakeRotator` (`KismetMathLibrary.RandomFloatInRange` _returnvalue_2 _returnvalue) (`KismetMathLibrary.RandomFloatInRange` _returnvalue_2 _returnvalue) (`KismetMathLibrary.RandomFloatInRange` _returnvalue_2 _returnvalue))) Start)))

(fn `From A to B`
  (params (A :type "Vector Structure") (B :type "Vector Structure") (`Accuracy MOA` :type "Float (double-precision)" :default 0.0) (Complex :type Boolean) (ActorsToIgnore :type "Array of Actor Object Reference (by ref)"))
  (returns (`Hit Any` :type Boolean) (Hit :type "HitResult Structure (by ref)") (Hits :type "Array of HitResult Structure"))
  (bind (_outhits _returnvalue) (`KismetSystemLibrary.LineTraceMultiForObjects` A (`self.Calculate Accuracy` A B `Accuracy MOA`) (`|MakeArray` "ObjectTypeQuery1" "ObjectTypeQuery2" "ObjectTypeQuery3" :!type "EObjectTypeQuery Enum") Complex ActorsToIgnore (select `bool` (`self.Show Traces`) :`true` "ForDuration" :!type "EDrawDebugTrace Enum") true (struct :`G` 0.620294 :`B` 1.0 :`A` 1.0) (struct :`B` 1.0 :`A` 1.0) 1.0))
  (if _returnvalue
    (return true (`|GetArrayItem` _outhits) _outhits)
    (else
      (return false))))

(fn `From Center Ranged`
  (params (`Interaction Type` :type "/Game/AdditionalContent/Project_Modular_GBS/Blueprints/Systems/Systems_Setup/Trace_Type Enum" :default "NewEnumerator1") (Complex :type Boolean) (`Custom Range` :type Boolean) (Range :type "Float (double-precision)") (ActorsToIgnore :type "Array of Actor Object Reference (by ref)"))
  (returns (`Hit Any` :type Boolean) (Hit :type "HitResult Structure (by ref)") (Hits :type "Array of HitResult Structure"))
  (bind (_start _rotation) (`self.Trace Start`))
  (bind (_outhits _returnvalue) (`KismetSystemLibrary.LineTraceMultiForObjects` _start (+ _start (* (`KismetMathLibrary.GetForwardVector` _rotation) (`KismetMathLibrary.SelectFloat` Range (`self.Default Range`) `Custom Range`))) (`|MakeArray` "ObjectTypeQuery1" "ObjectTypeQuery2" "ObjectTypeQuery3" :!type "EObjectTypeQuery Enum") Complex ActorsToIgnore (select `bool` (`self.Show Traces`) :`true` "ForDuration" :!type "EDrawDebugTrace Enum") true (struct :`G` 0.620294 :`B` 1.0 :`A` 1.0) (struct :`B` 1.0 :`A` 1.0) 1.0))
  (if _returnvalue
    (return true (`|GetArrayItem` _outhits) _outhits)
    (else
      (return false))))

(fn `From Point To Crosshair`
  (params (Start :type "Vector Structure") (Complex :type Boolean) (`Accuracy (MOA)` :type "Float (double-precision)") (Range :type "Float (double-precision)") (ActorsToIgnore :type "Array of Actor Object Reference (by ref)"))
  (returns (ReturnValue :type Boolean) (Hit :type "HitResult Structure (by ref)") (Hits :type "Array of HitResult Structure"))
  (locals (`End Location` :type "Vector Structure"))
  (bind _start (`local.Start`))
  (bind (_hit_any _hit) (`self.From Center Ranged` "NewEnumerator1" Complex true Range ActorsToIgnore))
  (set `local.End Location` (+ (* (`KismetMathLibrary.Normal` (- (`KismetMathLibrary.SelectVector` (`.Location` (`GameplayStatics.BreakHitResult` _hit)) (+ Start (* Range (`KismetMathLibrary.GetForwardVector` (`.Rotation` (`self.Trace Start`))))) _hit_any) _start)) (`local.Range`) 1.0) _start))
  (bind (_outhits _returnvalue) (`KismetSystemLibrary.LineTraceMultiForObjects` (`local.Start`) (`self.Calculate Accuracy` (`local.Start`) (`local.End Location`) (`local.Accuracy (MOA)`)) (`|MakeArray` "ObjectTypeQuery1" "ObjectTypeQuery2" "ObjectTypeQuery3" :!type "EObjectTypeQuery Enum") (`local.Complex`) (`local.ActorsToIgnore`) (select `bool` (`self.Show Traces`) :`true` "ForDuration" :!type "EDrawDebugTrace Enum") true (struct :`R` 1.0 :`G` 0.587562 :`A` 1.0) (struct :`R` 0.744792 :`G` 0.209539 :`A` 1.0) 1.0))
  (if _returnvalue
    (return true (`|GetArrayItem` _outhits) _outhits)
    (else
      (return false))))

(fn `Trace From A to B`
  (params (Start :type "Vector Structure") (End :type "Vector Structure") (Accuracy :type "Float (double-precision)") (Complex :type Boolean) (Ignore :type "Array of Actor Object Reference (by ref)"))
  (returns (`Hit Any` :type Boolean) (Hit :type "HitResult Structure") (Hits :type "Array of HitResult Structure"))
  (bind (_hit_any _hit _hits) (`self.From A to B` Start End Accuracy Complex Ignore))
  (return _hit_any _hit _hits))

(fn `Trace From Center Ranged`
  (params (`Interaction Type` :type "/Game/AdditionalContent/Project_Modular_GBS/Blueprints/Systems/Systems_Setup/Trace_Type Enum" :default "NewEnumerator1") (Complex :type Boolean) (`Custom Range` :type Boolean) (Range :type "Float (double-precision)") (`Actors To Ignore` :type "Array of Actor Object Reference (by ref)"))
  (returns (`Hit Any` :type Boolean) (Hit :type "HitResult Structure") (Hits :type "Array of HitResult Structure"))
  (bind (_hit_any _hit _hits) (`self.From Center Ranged` `Interaction Type` Complex `Custom Range` Range `Actors To Ignore`))
  (return _hit_any _hit _hits))

(fn `Trace From Point To Crosshair`
  (params (Start :type "Vector Structure") (Complex :type Boolean) (Accuracy :type "Float (double-precision)") (Range :type "Float (double-precision)") (`Actor to Ignore` :type "Array of Actor Object Reference (by ref)"))
  (returns (`Hit Any` :type Boolean) (Hit :type "HitResult Structure") (Hits :type "Array of HitResult Structure"))
  (bind (_returnvalue _hit _hits) (`self.From Point To Crosshair` Start Complex Accuracy Range `Actor to Ignore`))
  (return _returnvalue _hit _hits))

(fn `Trace Start`
  (returns (Start :type "Vector Structure") (Rotation :type "Rotator Structure"))
  (bind _returnvalue (`self.GetOwner`))
  (bind _returnvalue_2 (`Actor.GetComponentByClass` _returnvalue "/Script/Engine.CameraComponent"))
  (bind (_returnvalue_location _returnvalue_rotation) (`KismetMathLibrary.BreakTransform` (`Actor.GetTransform` _returnvalue)))
  (bind (_returnvalue_location_2 _returnvalue_rotation_2) (`KismetMathLibrary.BreakTransform` (`SceneComponent.K2_GetComponentToWorld` _returnvalue_2)))
  (bind _instigator (`Actor.Instigator` (`self.GetOwner`))
    (:`then`
      (bind (_returnvalue_location_3 _returnvalue_rotation_3) (`KismetMathLibrary.BreakTransform` (`SceneComponent.K2_GetComponentToWorld` (`Actor.GetComponentByClass` _instigator "/Script/Engine.CameraComponent"))))
      (return _returnvalue_location_3 _returnvalue_rotation_3))
    (:`else`
      (`/Engine/EditorBlueprintResources/StandardMacros.IsValid` _returnvalue_2
        (:`Is Valid`
          (return _returnvalue_location_2 _returnvalue_rotation_2))
        (:`Is Not Valid`
          (return _returnvalue_location _returnvalue_rotation))))))