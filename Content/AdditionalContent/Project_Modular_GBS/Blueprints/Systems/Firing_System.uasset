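; Firing_System is a weapon component that handles firing, ammo and reloading for its owning item, configured by a FiringData asset.
; TryFire gates shots on cooldown, trigger release and ammo, supporting single, automatic and timer-chained burst fire.
; Each shot plays sound, spends ammo, messages the owner and optionally adds recoil to control pitch.
; Cancellable timed reloads consume ammo from the instigator's Container_System; shotgun and charge data are only cached.
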(event `self.ReceiveBeginPlay`
  (`self.Update System data` (`self.Firing_Data`)))

(event `/Game/AdditionalContent/Project_Modular_GBS/Blueprints/Interfaces/BPI_Firing.Try Stop Fire`
  (set `self.Released` true))

(event `/Game/AdditionalContent/Project_Modular_GBS/Blueprints/Interfaces/BPI_Firing.Update Firing Data`
  (params (`New Data` :type "/Game/AdditionalContent/Project_Modular_GBS/Blueprints/Systems/Systems_Setup/DA_Weapon Object Reference"))
  (`self.Update System data` `New Data`))

(event `Start Reload`
  (bind (_base_fire_data_ammotype _base_fire_data_magazine _base_fire_data_shotscountperfire _base_fire_data_automatic _base_fire_data_firerate _base_fire_data_accuracymoa _base_fire_data_range _base_fire_data_damage _base_fire_data_recoil _base_fire_data_reloadtime) (break `/Game/AdditionalContent/Project_Modular_GBS/Blueprints/Systems/Systems_Setup/S_Base_Fire_Data` (`self.Base Fire Data`)))
  ;[1 1 1] Comment
  (if (not (`KismetSystemLibrary.K2_TimerExistsHandle` (`self.Reload Timer`)))
    (bind _returnvalue (`KismetSystemLibrary.K2_SetTimerDelegate` (`|CreateDelegate` :!event `Reload`) _base_fire_data_reloadtime))
    (set `self.Reload Timer` _returnvalue)
    (set `self.Reloading` true)))

(event `Cancel Reload`
  ;[1 1 1] Comment
  (`KismetSystemLibrary.K2_ClearAndInvalidateTimerHandle` (`self.Reload Timer`))
  (set `self.Reloading` false))

(fn `Burst Fire`
  (bind (_burst_fire_data_burst _burst_fire_data_burstcount _burst_fire_data_burstintervale) (break `/Game/AdditionalContent/Project_Modular_GBS/Blueprints/Systems/Systems_Setup/S_Burst_Fire_Data` (`self.Burst Fire Data`)))
  (if (or (== (`self.Burset Tracker`) 0) (== (`self.Current Ammo`) 0))
    (set `self.Just Fired` false)
    (else
      (`self.Fire`)
      (`KismetSystemLibrary.K2_SetTimerDelegate` (`|CreateDelegate` :!event `Burst Fire`) _burst_fire_data_burstintervale)
      (`/Engine/EditorBlueprintResources/StandardMacros.DecrementInt` (`self.Burset Tracker`)
        (:`  `
          _))))
  (return))

(fn `Can Reload`
  (returns (Available :type Integer) (Yes :type Boolean))
  (bind _base_fire_data_ammotype (break `/Game/AdditionalContent/Project_Modular_GBS/Blueprints/Systems/Systems_Setup/S_Base_Fire_Data` (`self.Base Fire Data`)))
  (for _array_element (`Actor.K2_GetComponentsByClass` (`Actor.Instigator` (`self.GetOwner`)) "/Game/AdditionalContent/Project_Modular_GBS/Blueprints/Systems/Container_System.Container_System_C")
    (bind _available (message `/Game/AdditionalContent/Project_Modular_GBS/Blueprints/Interfaces/BPI_Container.Query Item` _array_element _base_fire_data_ammotype (`self.Target Containers`)))
    (return _available (> _available 0))))

(fn `Enable Fire`
  (set `self.Can  Fire` true))

(fn `Fire`
  (returns (Fired :type Boolean))
  (bind _returnvalue (`self.GetOwner`))
  (bind (_ammotype _magazine _shotscountperfire _automatic _firerate _accuracymoa _range _damage _recoil _reloadtime _firesound) (break `/Game/AdditionalContent/Project_Modular_GBS/Blueprints/Systems/Systems_Setup/S_Base_Fire_Data` (`self.Base Fire Data`)))
  (bind _instigator (`Actor.Instigator` _returnvalue))
  (bind _returnvalue_2 (`Pawn.GetController` _instigator))
  (bind (_returnvalue_roll _returnvalue_pitch _returnvalue_yaw) (`KismetMathLibrary.BreakRotator` (`Pawn.GetControlRotation` _instigator)))
  (`GameplayStatics.PlaySoundAtLocation` _firesound (`Actor.K2_GetActorLocation` (`self.GetOwner`)) (struct) 1.0 1.0 0.0 null null null null)
  (bind _output_get (set `self.Current Ammo` (- (stale _output_get) (`KismetMathLibrary.SelectInt` 0 _shotscountperfire (`self.Infinit Magazine`)))))
  (set `self.Can  Fire` false)
  (message `/Game/AdditionalContent/Project_Modular_GBS/Blueprints/Interfaces/BPI_Weapon.Fired` _returnvalue)
  (set `self.Just Fired` true)
  (if (`self.Recoil`)
    (`/Engine/EditorBlueprintResources/StandardMacros.IsValid` _returnvalue_2
      (:`Is Valid`
        (`Controller.SetControlRotation` _returnvalue_2 (`KismetMathLibrary.MakeRotator` _returnvalue_roll (+ _returnvalue_pitch _recoil) _returnvalue_yaw)))
      (:`Is Not Valid`
        _))
    (return true)
    (else
      (return true))))

(fn `Reload`
  (locals (Reloaded :type Boolean))
  (bind (_ammo_type _quantity) (`self.Reload Request`))
  (for _array_element (`Actor.K2_GetComponentsByClass` (`Actor.Instigator` (`self.GetOwner`)) "/Game/AdditionalContent/Project_Modular_GBS/Blueprints/Systems/Container_System.Container_System_C")
    (bind _granted (message `/Game/AdditionalContent/Project_Modular_GBS/Blueprints/Interfaces/BPI_Container.Consume Request` _array_element _ammo_type _quantity true (`|MakeArray` "NewEnumerator3" :!type "/Game/AdditionalContent/Project_Modular_GBS/Blueprints/Systems/Systems_Setup/E_Container_Type Enum")))
    (bind _output_get (set `self.Current Ammo` (+ (stale _output_get) _granted)))
    (message `/Game/AdditionalContent/Project_Modular_GBS/Blueprints/Interfaces/BPI_Item.Item Quantity Updated` (`self.GetOwner`))
    (set `self.Reloading` false)
    (return))
  (set `self.Reloading` false)
  (return))

(fn `Reload Request`
  (returns (`Ammo Type` :type "/Game/AdditionalContent/Project_Modular_GBS/Blueprints/Systems/Systems_Setup/DA_Item Object Reference") (Quantity :type Integer))
  (bind (_ammotype _magazine) (break `/Game/AdditionalContent/Project_Modular_GBS/Blueprints/Systems/Systems_Setup/S_Base_Fire_Data` (`self.Base Fire Data`)))
  (return _ammotype (- _magazine (`self.Current Ammo`))))

(fn `Start Fire Timer`
  (locals (NewLocalVar :type "TimerHandle Structure"))
  (bind (_burst_fire_data_burst _burst_fire_data_burstcount _burst_fire_data_burstintervale) (break `/Game/AdditionalContent/Project_Modular_GBS/Blueprints/Systems/Systems_Setup/S_Burst_Fire_Data` (`self.Burst Fire Data`)))
  (bind (_ammotype _magazine _shotscountperfire _automatic _firerate) (break `/Game/AdditionalContent/Project_Modular_GBS/Blueprints/Systems/Systems_Setup/S_Base_Fire_Data` (`self.Base Fire Data`)))
  (`KismetSystemLibrary.K2_SetTimerDelegate` (`|CreateDelegate` :!event `Enable Fire`) (`KismetMathLibrary.SelectFloat` (+ _firerate (* _burst_fire_data_burstcount _burst_fire_data_burstintervale)) _firerate _burst_fire_data_burst))
  (return))

(fn `Stop Fire`)

(fn `Try Fire`
  (returns (Fired :type Boolean))
  (bind _fired (`self.Try Firing`))
  (return _fired))

(fn `Try Firing`
  (returns (Fired :type Boolean))
  (bind (_burst_fire_data_burst _burst_fire_data_burstcount) (break `/Game/AdditionalContent/Project_Modular_GBS/Blueprints/Systems/Systems_Setup/S_Burst_Fire_Data` (`self.Burst Fire Data`)))
  (set `self.Just Fired` false)
  (if (`self.Can  Fire`)
    (if (`self.Released`)
      (if (> (`self.Current Ammo`) 0)
        (if (not _burst_fire_data_burst)
          (`self.Fire`)
          (else
            (set `self.Burset Tracker` _burst_fire_data_burstcount)
            (`self.Burst Fire`)))
        (`self.Start Fire Timer`)
        (if (not (`.Automatic_24_87B1095A43B5D63A9B790BB7015FE092` (break `/Game/AdditionalContent/Project_Modular_GBS/Blueprints/Systems/Systems_Setup/S_Base_Fire_Data` (`self.Base Fire Data`))))
          (set `self.Released` false))
        (return (`self.Just Fired`))))))

(fn `Update System data`
  (params (Target :type "/Game/AdditionalContent/Project_Modular_GBS/Blueprints/Systems/Systems_Setup/DA_Weapon Object Reference"))
  (bind (_ammotype _magazine) (break `/Game/AdditionalContent/Project_Modular_GBS/Blueprints/Systems/Systems_Setup/S_Base_Fire_Data` (`self.Base Fire Data`)))
  (`/Engine/EditorBlueprintResources/StandardMacros.IsValid` Target
    (:`Is Valid`
      (bind _output_get (set `self.Firing_Data` Target))
      (set `self.Base Fire Data` (`/Game/AdditionalContent/Project_Modular_GBS/Blueprints/Systems/Systems_Setup/DA_Weapon.Base` _output_get))
      (set `self.Burst Fire Data` (`/Game/AdditionalContent/Project_Modular_GBS/Blueprints/Systems/Systems_Setup/DA_Weapon.Burst` _output_get))
      (set `self.Shotgun Fire Data` (`/Game/AdditionalContent/Project_Modular_GBS/Blueprints/Systems/Systems_Setup/DA_Weapon.Shotgun` _output_get))
      (set `self.Charge Fire Data` (`/Game/AdditionalContent/Project_Modular_GBS/Blueprints/Systems/Systems_Setup/DA_Weapon.Charge` _output_get))
      (if (`self.Start With Full Magazine`)
        (set `self.Current Ammo` _magazine)
        (else
          (bind _output_get_2 (set `self.Current Ammo` (`KismetMathLibrary.Clamp` (stale _output_get_2) 0 _magazine))))))))