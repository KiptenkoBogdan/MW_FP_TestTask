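; Demo actor for the TraceSystem in Project Modular GBS that displays what a point-to-point trace hits.
; An overlap on its Sphere calls Apply after a short retriggerable delay, which traces from the root to TraceEnd through TraceSystem.FromAToB.
; On any hit, the TextRender shows the hit actor.
; The construction script moves TraceEnd to the relative TraceTarget location.
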(event `Apply`
  (bind (_hit_any _hit) (`/Game/AdditionalContent/Project_Modular_GBS/Blueprints/Systems/Trace_System.From A to B` :`self` (`self.Trace_System`) :`A` (`SceneComponent.K2_GetComponentLocation` (`self.DefaultSceneRoot`)) :`B` (`SceneComponent.K2_GetComponentLocation` (`self.Trace End`))))
  (if _hit_any
    (`TextRenderComponent.K2_SetText` (`self.TextRender`) (`KismetTextLibrary.Conv_ObjectToText` (`.HitActor` (`GameplayStatics.BreakHitResult` _hit))))))

(event `self.Sphere.OnComponentBeginOverlap`
  (params (OverlappedComponent :type "PrimitiveComponent Object Reference") (OtherActor :type "Actor Object Reference") (OtherComp :type "PrimitiveComponent Object Reference") (OtherBodyIndex :type Integer) (bFromSweep :type Boolean) (SweepResult :type "HitResult Structure (by ref)"))
  (`KismetSystemLibrary.RetriggerableDelay` 0.1)
  (`self.Apply`))

(fn `UserConstructionScript`
  (`SceneComponent.K2_SetRelativeLocation` (`self.Trace End`) (`self.Trace Target`) false false))