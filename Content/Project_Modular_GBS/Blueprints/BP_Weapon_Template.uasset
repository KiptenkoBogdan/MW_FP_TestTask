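; Template weapon item that turns use and reload input into firing, reloading and damage through modular components.
; Construction feeds the item's weapon data to FiringSystem, whose Fired event updates the widget, applies damage and cancels any reload.
; Each shot traces from the mesh toward the crosshair with MOA spread, with shotguns tracing per pellet and splitting damage.
; Equip and unequip toggle visibility and input, with unequip also cancelling reloads.
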(event `EnhancedInput|/Game/FirstPerson/Input/Actions/IA_Use`
  (params (ActionValue :type Boolean) (ElapsedSeconds :type "Float (double-precision)") (TriggeredSeconds :type "Float (double-precision)") (InputAction :type "InputAction Object Reference" :default "/Game/FirstPerson/Input/Actions/IA_Use.IA_Use"))
  (bind _firing_system (`self.Firing_System`))
  (:`Triggered`
    (message `/Game/Project_Modular_GBS/Blueprints/Interfaces/BPI_Firing.Try Fire` _firing_system))
  (:`Completed`
    (message `/Game/Project_Modular_GBS/Blueprints/Interfaces/BPI_Firing.Try Stop Fire` _firing_system)))

(event `EnhancedInput|/Game/Project_Modular_GBS/Blueprints/Player/Input/IA_Reload`
  (params (ActionValue :type Boolean) (ElapsedSeconds :type "Float (double-precision)") (TriggeredSeconds :type "Float (double-precision)") (InputAction :type "InputAction Object Reference" :default "/Game/Project_Modular_GBS/Blueprints/Player/Input/IA_Reload.IA_Reload"))
  (bind _firing_system (`self.Firing_System`))
  (:`Started`
    (if (and (`.Yes` (`/Game/Project_Modular_GBS/Blueprints/Systems/Firing_System.Can Reload` _firing_system)) (not (`/Game/Project_Modular_GBS/Blueprints/Systems/Firing_System.Reloading` _firing_system)))
      (`/Game/Project_Modular_GBS/Blueprints/Systems/Firing_System.Start Reload` _firing_system)
      (message `/Game/Project_Modular_GBS/Blueprints/Interfaces/BPI_Item.Start Timer` (`self.Item Widget`) (`.ReloadTime_16_E6EE7EE1441C8D2E55843CBE24EFBDDC` (break `/Game/Project_Modular_GBS/Blueprints/Systems/Systems_Setup/S_Base_Fire_Data` (`/Game/Project_Modular_GBS/Blueprints/Systems/Firing_System.Base Fire Data` _firing_system)))))))

(event `/Game/Project_Modular_GBS/Blueprints/Interfaces/BPI_Weapon.Fired`
  (`self.Update Widget`)
  (`self.Send damage`)
  (`/Game/Project_Modular_GBS/Blueprints/Systems/Firing_System.Cancel Reload` (`self.Firing_System`))
  (message `/Game/Project_Modular_GBS/Blueprints/Interfaces/BPI_Item.Cancel Timer` (`self.Item Widget`)))

(event `/Game/Project_Modular_GBS/Blueprints/Interfaces/BPI_Item.Equip Item`
  (`self.SetActorHiddenInGame` false)
  (`self.EnableInput` (`GameplayStatics.GetPlayerController` 0)))

(event `/Game/Project_Modular_GBS/Blueprints/Interfaces/BPI_Item.UnEquip Item`
  (`/Game/Project_Modular_GBS/Blueprints/Systems/Firing_System.Cancel Reload` (`self.Firing_System`))
  (`self.SetActorHiddenInGame` true)
  (`self.DisableInput` (`GameplayStatics.GetPlayerController` 0))
  (message `/Game/Project_Modular_GBS/Blueprints/Interfaces/BPI_Interact.Hide All Interactions` (`self.GetComponentByClass` (`self.Instigator`) "/Game/Project_Modular_GBS/Blueprints/Systems/Interaction_System.Interaction_System_C") true)
  (message `/Game/Project_Modular_GBS/Blueprints/Interfaces/BPI_Item.Cancel Timer` (`self.Item Widget`)))

(fn `Send damage`
  (bind _firing_system (`self.Firing_System`))
  (bind _firing_system_2 (`self.Firing_System`))
  (bind (_ammotype _magazine _shotscountperfire _automatic _firerate _accuracymoa _range) (break `/Game/Project_Modular_GBS/Blueprints/Systems/Systems_Setup/S_Base_Fire_Data` (`/Game/Project_Modular_GBS/Blueprints/Systems/Firing_System.Base Fire Data` _firing_system_2)))
  (bind (_shotgun _shotspershell) (break `/Game/Project_Modular_GBS/Blueprints/Systems/Systems_Setup/S_Shotgun_Fire_Data` (`/Game/Project_Modular_GBS/Blueprints/Systems/Firing_System.Shotgun Fire Data` _firing_system_2)))
  (bind (_ammotype_2 _magazine_2 _shotscountperfire_2 _automatic_2 _firerate_2 _accuracymoa_2 _range_2 _damage) (break `/Game/Project_Modular_GBS/Blueprints/Systems/Systems_Setup/S_Base_Fire_Data` (`/Game/Project_Modular_GBS/Blueprints/Systems/Firing_System.Base Fire Data` _firing_system)))
  (bind (_shotgun_2 _shotspershell_2) (break `/Game/Project_Modular_GBS/Blueprints/Systems/Systems_Setup/S_Shotgun_Fire_Data` (`/Game/Project_Modular_GBS/Blueprints/Systems/Firing_System.Shotgun Fire Data` _firing_system)))
  (for _ (range 1 (+ (select `bool` _shotgun :`false` 1 :`true` _shotspershell) 1))
    (bind (_returnvalue _hit) (`/Game/Project_Modular_GBS/Blueprints/Systems/Trace_System.From Point To Crosshair` (`self.Trace_System`) (`SceneComponent.K2_GetComponentLocation` (`self.Static Mesh`)) true _accuracymoa (* _range 100.0) (`|MakeArray` self (`self.Instigator`) :!type "Actor Object Reference")))
    (if _returnvalue
      (`/Game/Project_Modular_GBS/Blueprints/Systems/Damage_System.Damage` (`self.Damage_System`) (`.HitActor` (`GameplayStatics.BreakHitResult` _hit)) "NewEnumerator4" (`KismetMathLibrary.SelectFloat` (/ _damage _shotspershell_2) _damage _shotgun_2) (`self.Instigator`)))))

(fn `UserConstructionScript`
  (`parent.UserConstructionScript`)
  (message `/Game/Project_Modular_GBS/Blueprints/Interfaces/BPI_Firing.Update Firing Data` (`self.Firing_System`) (`/Game/Project_Modular_GBS/Blueprints/Systems/Systems_Setup/DA_Item.Weapon Data` (`self.Item Data`))))