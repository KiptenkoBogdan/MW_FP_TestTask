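; Interactable target range switch that spawns BP_NPC targets at random offsets from a spawner location while active.
; Interact toggles the spawn timer, cube material and context label, and resets the player's score message on activation.
; Player score increases shorten the interval down to a floor, and each spawn re-sets the timer to apply it.
; Tick drives the label's countdown progress, and each NPC's despawn time derives from the current and base intervals.
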(event `self.ReceiveBeginPlay`
  (bind _returnvalue (`GameplayStatics.GetActorOfClass` "/Game/PlayerCharacter/Blueprints/Player/ThirdPersonCharacter.ThirdPersonCharacter_C"))
  (add `/Game/PlayerCharacter/Blueprints/Player/ThirdPersonCharacter.OnScoreIncreased` _returnvalue (delegate `Decrease Timer`))
  (bind _aswbp_context_label (cast `/Game/PlayerCharacter/Blueprints/Player/Widgets/WBP_ContextLabel` (`WidgetComponent.GetWidget` (`self.Widget`))))
  (`/Game/PlayerCharacter/Blueprints/Player/Widgets/WBP_ContextLabel.fSetText` _aswbp_context_label "Target Range OFF"))

(event `Decrease Timer`
  (bind _returnvalue (- (`self.BaseTime`) (/ (`/Game/PlayerCharacter/Blueprints/Player/ThirdPersonCharacter.Score` (stale `self.ReceiveBeginPlay` _returnvalue)) 10)))
  (if (>= _returnvalue 0.5)
    (bind _output_get (set `self.Time` _returnvalue))
    (`KismetSystemLibrary.PrintString` (`KismetStringLibrary.Conv_DoubleToString` _output_get))))

(event `self.ReceiveTick`
  (params (DeltaSeconds :type "Float (single-precision)"))
  (`self.TimerProgress`))

(event `/Game/PlayerCharacter/Interfaces/BPI_Interactable.Interact`
  (bind _output_get (set `self.IsActive` (not (`self.IsActive`))))
  (if _output_get
    (message `/Game/PlayerCharacter/Blueprints/Player/BPI_Score.ResetScore` (`GameplayStatics.GetPlayerCharacter` 0))
    (`PrimitiveComponent.SetMaterial` (`self.Cube`) 0 "/Engine/MapTemplates/Materials/BasicAsset03.BasicAsset03")
    (bind _aswbp_context_label (cast `/Game/PlayerCharacter/Blueprints/Player/Widgets/WBP_ContextLabel` (`WidgetComponent.GetWidget` (`self.Widget`))))
    (`/Game/PlayerCharacter/Blueprints/Player/Widgets/WBP_ContextLabel.fSetText` _aswbp_context_label "Target Range ON")
    (bind _returnvalue (`KismetSystemLibrary.K2_SetTimerDelegate` (delegate `Spawn Targets`) (`self.Time`) true :!label _label))
    (set `self.TimerHandle` _returnvalue)
    (`self.ResetTimer`)
    (else
      (`PrimitiveComponent.SetMaterial` (`self.Cube`) 0 "/Engine/BasicShapes/BasicShapeMaterial.BasicShapeMaterial")
      (`KismetSystemLibrary.K2_PauseTimerHandle` (`self.TimerHandle`))
      (bind _aswbp_context_label_2 (cast `/Game/PlayerCharacter/Blueprints/Player/Widgets/WBP_ContextLabel` (`WidgetComponent.GetWidget` (`self.Widget`))))
      (`/Game/PlayerCharacter/Blueprints/Player/Widgets/WBP_ContextLabel.fSetText` _aswbp_context_label_2 "Target Range OFF"))))

(event `Spawn Targets`
  (`self.SpawnNPC`)
  (`self.ResetTimer`)
  (goto _label))

(event `TimerProgress`
  (bind _output_get (set `self.TimerCountdownTime` (`KismetMathLibrary.FClamp` (- (`self.TimerCountdownTime`) (`GameplayStatics.GetWorldDeltaSeconds`)) 0.0 (`self.TimerCountdownTime`))))
  (bind _aswbp_context_label (cast `/Game/PlayerCharacter/Blueprints/Player/Widgets/WBP_ContextLabel` (`WidgetComponent.GetWidget` (`self.Widget`))))
  (`/Game/PlayerCharacter/Blueprints/Player/Widgets/WBP_ContextLabel.fSetTimerProgress` _aswbp_context_label (`KismetMathLibrary.NormalizeToRange` _output_get 0.0 (`self.Time`))))

(event `ResetTimer`
  (set `self.TimerCountdownTime` (`self.Time`)))

(fn `SpawnNPC`
  (`|SpawnActorFromClass` "/Game/PlayerCharacter/NPC/BP_NPC.BP_NPC_C" (`KismetMathLibrary.MakeTransform` (+ (`self.SpawnerLocalion`) (`KismetMathLibrary.MakeVector` 0.0 (`KismetMathLibrary.RandomFloatInRange` 0.0 800.0) (`KismetMathLibrary.RandomFloatInRange` -100.0 600.0)))) "Undefined" "MultiplyWithRoot" null (+ (`self.Time`) (`self.BaseTime`)) null))

(fn `UserConstructionScript`)