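; Enemy AI character that roams, chases the player and ragdolls before being destroyed on death.
; Roaming is a self-restarting loop of AI moves to random reachable points with random pauses.
; Seeing a pawn or being hit runs the MChasePlayer macro, which speeds it up and moves it toward the target.
; A retriggerable delay in that macro returns it to slow roaming shortly after the last trigger.
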(event `ChasePlayer`)

(event `self.ReceiveBeginPlay`
  (set `CharacterMovementComponent.MaxWalkSpeed` 200.0 (`self.CharacterMovement`))
  (`KismetSystemLibrary.Delay` 3.0)
  (`self.Roam`))

(event `Roam`
  (if (`self.IsRoaming`)
    (`|AIMoveTo` self (`NavigationSystemV1.K2_GetRandomReachablePointInRadius` (`self.K2_GetActorLocation`) 1500.0 null null) null 0.0
      (:`OnSuccess`
        _)
      (:`OnFail`
        _))
    (`KismetSystemLibrary.Delay` (`KismetMathLibrary.RandomFloatInRange` 1.0 4.0))
    (`self.Roam`)))

(event `/Game/PlayerCharacter/Interfaces/BPI_NPC.OnHit`
  (bind _outactors (`GameplayStatics.GetAllActorsOfClass` "/Game/PlayerCharacter/Blueprints/Player/ThirdPersonCharacter.ThirdPersonCharacter_C"))
  (`self.MChasePlayer` (`|GetArrayItem` _outactors)))

(event `/Game/PlayerCharacter/Interfaces/BPI_NPC.Death`
  (`PrimitiveComponent.SetSimulatePhysics` (`self.Mesh`) true)
  (`CharacterMovementComponent.DisableMovement` (`self.CharacterMovement`))
  (`KismetSystemLibrary.PrintString` "Enemy killed")
  (`KismetSystemLibrary.Delay` 3.0)
  (`self.K2_DestroyActor`))

(event `self.PawnSensing.OnSeePawn`
  (params (Pawn :type "Pawn Object Reference"))
  (`self.MChasePlayer` Pawn))

(fn `UserConstructionScript`)