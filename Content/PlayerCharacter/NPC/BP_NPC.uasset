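; BP_NPC is a target character that the player scores by hitting before it despawns.
; A timer started at BeginPlay calls DeathEvent on its health manager component after DespawnTime.
; OnHit swaps the sphere material, marks it activated, plays a ping and calls AddScoreMessage on the player character.
; Death destroys the actor and plays a failure sound if it was never activated.
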(event `self.ReceiveBeginPlay`
  (`KismetSystemLibrary.Delay` (`self.DespawnTime`))
  (`/Game/PlayerCharacter/Components/AC_HealthManager.DeathEvent` (`self.AC_HealthManager`)))

(event `/Game/PlayerCharacter/Interfaces/BPI_NPC.Death`
  (`self.K2_DestroyActor`)
  (`KismetSystemLibrary.PrintString` "Enemy killed")
  (if (not (`self.IsActivated`))
    (`GameplayStatics.PlaySound2D` "/Engine/EditorSounds/Notifications/CompileFailed.CompileFailed" 1.0 1.0 0.0 null null)))

(event `/Game/PlayerCharacter/Interfaces/BPI_NPC.OnHit`
  (`PrimitiveComponent.SetMaterial` (`self.Sphere`) 0 "/Engine/MapTemplates/Materials/BasicAsset03.BasicAsset03")
  (set `self.IsActivated` true)
  (`GameplayStatics.PlaySound2D` "/Engine/EngineSounds/1kSineTonePing.1kSineTonePing" 1.0 1.0 0.0 null null)
  (message `/Game/PlayerCharacter/Blueprints/Player/BPI_Score.AddScore` (`GameplayStatics.GetPlayerCharacter` 0)))

(fn `UserConstructionScript`)