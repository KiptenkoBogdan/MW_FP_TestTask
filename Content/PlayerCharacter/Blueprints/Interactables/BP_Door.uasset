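; BP_Door is an interactable double sliding door that toggles between open and closed.
; Interact moves the left and right panels in opposite directions by a fixed local offset and flips IsClosed, snapping instantly with no animation or sweep.
; ShowContextClue uses the same flag to pass the open or close prompt to the supplied HUD widget.
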(event `/Game/PlayerCharacter/Interfaces/BPI_Interactable.ShowContextClue`
  (params (HUDWidget :type "/Game/PlayerCharacter/Blueprints/Player/Widgets/WBP_HUD Object Reference"))
  ;[1 1 1] Show Context Clue
  (if (`self.IsClosed`)
    (`/Game/PlayerCharacter/Blueprints/Player/Widgets/WBP_HUD.fShowContextClue` HUDWidget (`self.ContextClueOpen`))
    (else
      (`/Game/PlayerCharacter/Blueprints/Player/Widgets/WBP_HUD.fShowContextClue` HUDWidget (`self.ContextClueClosed`)))))

(event `/Game/PlayerCharacter/Interfaces/BPI_Interactable.Interact`
  ;[1 1 1] Intecraction
  (if (`self.IsClosed`)
    (`SceneComponent.K2_AddLocalOffset` (`self.RightDoor`) (150.0 0.0 0.0) false false)
    (`SceneComponent.K2_AddLocalOffset` (`self.LeftDoor`) (-150.0 0.0 0.0) false false)
    (set `self.IsClosed` false)
    (else
      (`SceneComponent.K2_AddLocalOffset` (`self.RightDoor`) (-150.0 0.0 0.0) false false)
      (`SceneComponent.K2_AddLocalOffset` (`self.LeftDoor`) (150.0 0.0 0.0) false false)
      (set `self.IsClosed` true))))

(fn `UserConstructionScript`)