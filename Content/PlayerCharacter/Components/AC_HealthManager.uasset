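; AC_HealthManager is an actor component that tracks health and handles death for its owning actor.
; FRemoveHealth subtracts the given amount from TargetHealth, prints the new value, and fires DeathEvent when it reaches zero or below.
; DeathEvent sends DeathMessage to the owner only if it implements the BPI_NPC interface, leaving the death response to that actor.
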(event `DeathEvent`
  (bind _returnvalue (`self.GetOwner`))
  (if (`KismetSystemLibrary.DoesImplementInterface` _returnvalue "/Game/PlayerCharacter/Interfaces/BPI_NPC.BPI_NPC_C")
    (message `/Game/PlayerCharacter/Interfaces/BPI_NPC.Death` _returnvalue)))

(fn `fRemoveHealth`
  (params (NewAmount :type "Float (double-precision)"))
  (bind _output_get (set `self.TargetHealth` (- (`self.TargetHealth`) NewAmount)))
  ;[1 1 1] On HP Removed Message
  (`KismetSystemLibrary.PrintText` (`KismetTextLibrary.Conv_DoubleToText` _output_get "HalfToEven"))
  (if (<= _output_get 0.0)
    (`self.DeathEvent`)))